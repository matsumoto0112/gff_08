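; BP_Stalker is a follower actor that serves as the player's view target while shadowing another actor.
; On BeginPlay it stores the actor found for TargetClass as Target and switches player controller 0's view to itself.
; Every Tick it copies Target's location with a swept move and matches its rotation, with no smoothing, offset or validity check.
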(event EventBeginPlay
  (bind _returnvalue (Actor|GetActorOfClass (Variables|Default|GetTargetClass)))
  (Variables|Default|SetTarget _returnvalue)
  (Game|Player|SetViewTargetwithBlend (Game|GetPlayerController 0) self 0.0 "VTBlend_Linear" 0.0 false))

(event Collision|EventActorBeginOverlap
  (params (OtherActor :type Actor%20Object%20Reference)))

(event EventTick
  (params (DeltaSeconds :type Float%20%28single-precision%29))
  (bind _target (Variables|Default|GetTarget))
  (Transformation|SetActorLocation (Transformation|GetActorLocation _target) true false)
  (Transformation|SetActorRotation (Transformation|GetActorRotation _target)))

(fn ConstructionScript)