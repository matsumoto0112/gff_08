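; AI-driven boat that heads for its next checkpoint by setting left and right motor values each tick.
; A speed-scaled forward trace detects obstacles and triggers a hard turn, its side chosen by the 2D cross product toward the checkpoint.
; Otherwise, a second trace and that cross product select straight or gentler differential steering.
; It also draws debug lines and plays a sound on wall hits.
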(event OnComponentHit(StaticMesh)
  (params (HitComponent :type Primitive%20Component%20Object%20Reference) (OtherActor :type Actor%20Object%20Reference) (OtherComp :type Primitive%20Component%20Object%20Reference) (NormalImpulse :type Vector :default "0, 0, 0") (Hit :type Hit%20Result%20Structure%20%28by%20ref%29))
  (bind _asbp_wall_parent (Utilities|Casting|CastToBP_WallParent OtherActor))
  (bind _instance (CallFunction|GetMyGameInstance))
  (Class|SoundSystem|PlaySoundwithAttachOwnerActor (Class|MyGameInstance|GetSoundSystem _instance) "SE_BOAT_HIT" _asbp_wall_parent true))

(event EventBeginPlay
  (|CallParentFunction)
  (Rendering|Material|SetMaterial (Variables|Default|GetStaticMesh) 0 "/AnimationSharing/AnimSharingGreen.AnimSharingGreen"))

(event Collision|EventActorBeginOverlap
  (params (OtherActor :type Actor%20Object%20Reference))
  (|CallParentFunction OtherActor) ; This node is disabled and will not be called.\nDrag off pins to build functionality.
)

(event EventTick
  (params (DeltaSeconds :type Float%20%28single-precision%29))
  (|CallParentFunction DeltaSeconds)
  (CallFunction|PrinttoCheckPointLine)
  (bind _angle (CallFunction|GetCrosstoCheckPoint2d))
  (bind _find (CallFunction|FindObjecttoForward))
  (if _find ; 正面方向に障害物があるか
    (if (>= (Math|Trig|RadiansToDegrees _angle) 0.0)
      (CallFunction|SetMovementValues 0.0 0.8)
      (else
        (CallFunction|SetMovementValues 0.8 0.0)))
    (else
      ;[1 1 1] 障害物がなければチェックポイントの真ん中をできるだけ通過するようにする
      (bind _distance (CallFunction|GetDistancetoCheckPoint))
      (if (<= _distance 1e+02)
        (CallFunction|SetMovementValues 0.7 0.7 :!label _label)
        (else
          (bind _type (CallFunction|RangeCheck (Math|Trig|RadiansToDegrees _angle) -6e+01 6e+01))
          (switch Utilities|FlowControl|Switch|SwitchonBP_FloatRangeType _type
            (:NewEnumerator0
              (CallFunction|SetMovementValues 0.6 0.1))
            (:NewEnumerator1
              (goto _label))
            (:NewEnumerator2
              (CallFunction|SetMovementValues 0.1 0.6))))))))

(fn ConstructionScript
  (|CallParentFunction))

(fn PrinttoCheckPointLine
  (Rendering|Debug|DrawDebugLine (Transformation|GetActorLocation) (Transformation|GetActorLocation (Variables|Default|GetNextCheckPoint)) "(R=1.000000,G=0.034167,B=0.296308,A=1.000000)" 0.1 0.0))

(fn FindObjecttoForward
  (bind _returnvalue (Transformation|GetActorLocation))
  (bind _kilometerperhour (CallFunction|ToSpeedKilometerPerHour (Math|Vector|VectorLength (Transformation|GetVelocity))))
  (bind (_outhit _returnvalue_2) (Collision|LineTraceByChannel _returnvalue (+ _returnvalue (* (Transformation|GetActorForwardVector) (* _kilometerperhour 5e+01))) "TraceTypeQuery4" false 0 "ForOneFrame"))
  (return _returnvalue_2 _outhit))

(fn SetMovementValues
  (params (Left :type Float%20%28single-precision%29) (Right :type Float%20%28single-precision%29))
  (Variables|Default|SetLeftMotorValue Left)
  (Variables|Default|SetRightMotorValue Right))

(fn GetCrosstoCheckPoint2d
  (return (Class|KismetMathLibrary|CrossProduct2D (Math|Vector2D|Normalize2D (Math|Conversions|ToVector2D(Vector) (Transformation|GetActorForwardVector))) (Math|Vector2D|Normalize2D (Math|Conversions|ToVector2D(Vector) (- (Transformation|GetActorLocation (Variables|Default|GetNextCheckPoint)) (Transformation|GetActorLocation)))))))

(fn GetDistancetoCheckPoint
  (bind (_outhit _returnvalue) (Collision|LineTraceByChannel (Transformation|GetActorLocation) (+ (Transformation|GetActorLocation) (* (Transformation|GetActorForwardVector) 1e+03)) "TraceTypeQuery3" false 0 "ForOneFrame" true "(R=0.000000,G=0.243322,B=1.000000,A=1.000000)"))
  (return (Math|Float|SelectFloat (.Distance (Collision|BreakHitResult _outhit)) 1e+03 _returnvalue)))