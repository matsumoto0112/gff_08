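; BP_AIPlayer is an AI-driven actor that travels along a chain of BP_CheckPoint actors.
; Each Tick, MoveTo offsets it a fixed step toward NextCheckPoint on the XY plane, without sweep or delta-time scaling.
; When its StaticMesh overlaps a checkpoint, that checkpoint's GetNextPoint supplies the new target.
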(event OnComponentBeginOverlap(StaticMesh)
  (params (OverlappedComponent :type Primitive%20Component%20Object%20Reference) (OtherActor :type Actor%20Object%20Reference) (OtherComp :type Primitive%20Component%20Object%20Reference) (OtherBodyIndex :type Integer) (bFromSweep :type Boolean) (SweepResult :type Hit%20Result%20Structure%20%28by%20ref%29))
  (bind _asbp_check_point (Utilities|Casting|CastToBP_CheckPoint OtherActor))
  (bind _nextpoint (Default|GetNextPoint _asbp_check_point))
  (Variables|Default|SetNextCheckPoint _nextpoint))

(event EventBeginPlay)

(event Collision|EventActorBeginOverlap
  (params (OtherActor :type Actor%20Object%20Reference)))

(event EventTick
  (params (DeltaSeconds :type Float%20%28single-precision%29))
  (CallFunction|Moveto))

(fn ConstructionScript)

(fn Moveto
  (bind _returnvalue (Transformation|GetActorLocation))
  (bind _nextcheckpoint (Variables|Default|GetNextCheckPoint))
  (bind _returnvalue_2 (Transformation|GetActorLocation _nextcheckpoint))
  (bind _returnvalue_3 (- _returnvalue_2 _returnvalue))
  (bind _returnvalue_4 (Class|KismetMathLibrary|VectorNormal2D _returnvalue_3 0.0001))
  (bind _returnvalue_5 (* _returnvalue_4 10))
  (bind (_x _y) (Math|Vector|BreakVector _returnvalue_5))
  (Transformation|AddActorWorldOffset (Math|Vector|MakeVector _x _y 0.0)))