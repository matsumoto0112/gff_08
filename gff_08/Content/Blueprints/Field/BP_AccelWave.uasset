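; BP_AccelWave is a field actor that removes itself after a fixed lifetime of about ten seconds.
; BeginPlay passes the current time to Initialize, which stores it as StartTime.
; Tick compares the elapsed time against that stamp and destroys the actor once the limit is reached.
; The overlap event is a disabled stub, so the file itself contains no acceleration or interaction logic.
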(event EventBeginPlay
  (CallFunction|Initialize (Math|DateTime|Now)))

(event Collision|EventActorBeginOverlap
  (params (OtherActor :type Actor%20Object%20Reference)))

(event EventTick
  (params (DeltaSeconds :type Float%20%28single-precision%29))
  (if (>= (Math|Timespan|GetSeconds (- (Math|DateTime|Now) (Variables|Default|GetStartTime))) 10)
    (Actor|DestroyActor)))

(fn ConstructionScript)

(fn Initialize
  (params (NewParam :type Date%20Time%20Structure))
  (Variables|Default|SetStartTime NewParam))