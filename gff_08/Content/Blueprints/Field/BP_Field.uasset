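; BP_Field is the field actor that tracks acceleration waves on a 2D grid and supplies their push velocity by position, apparently for boats.
; On BeginPlay it reads its bounds and sizes a nested Row-by-Column wave array, with positions mapped to clamped cells assuming an origin-centered field.
; GenerateAccelWave spawns a BP_AccelWave only in an unoccupied cell, storing yaw-based direction, length and start time.
; GetAccelVelocity returns that cell's direction times length, or zero without a wave.
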(event EventBeginPlay
  (CallFunction|Initialize))

(event EventTick
  (params (DeltaSeconds :type Float%20%28single-precision%29)))

(fn ConstructionScript)

(fn Initialize
  (bind _boxextent (Collision|GetActorBounds false false))
  (bind (_x _y) (Math|Vector|BreakVector _boxextent))
  ;[1 1 1] Field Actorの幅と高さを取得する
  (bind _output_get (Variables|Default|SetWidth _x))
  (bind _output_get_2 (Variables|Default|SetHeight _y))
  (Development|PrintString (Utilities|String|ToString(Text) (Utilities|Text|FormatText "Width : {0}  Height : {1}" _output_get _output_get_2)))
  ;[1 1 1] 波情報の二重配列の初期化
  (Utilities|Array|Resize (Variables|Default|GetWaveArray) (Variables|Default|GetRow))
  (for (_ _array_index) (Variables|Default|GetWaveArray)
    (Utilities|Array|Resize (Utilities|Struct|BreakAccelWaveArray (Utilities|Array|Get(acopy) (Variables|Default|GetWaveArray) _array_index)) (Variables|Default|GetColumn))))

(fn GenerateAccelWave
  (params (spawnPosition :type Vector) (rotate :type Rotator))
  (LocalVariables|Setposition spawnPosition)
  (LocalVariables|Setrotation rotate)
  ;[1 1 1] グリッド座標を求める
  (LocalVariables|SetX (.X (Math|Vector|BreakVector (LocalVariables|Getposition))))
  (LocalVariables|SetY (.Y (Math|Vector|BreakVector (LocalVariables|Getposition))))
  (bind _value (CallFunction|CulcGrid (LocalVariables|GetX) (Variables|Default|GetWidth) (Variables|Default|GetRow)))
  (LocalVariables|Setgrid_row _value)
  (bind _value_2 (CallFunction|CulcGrid (LocalVariables|GetY) (Variables|Default|GetHeight) (Variables|Default|GetColumn)))
  (LocalVariables|Setgrid_column _value_2)
  (if (not (Utilities|IsValid (.WaveObject (Utilities|Struct|BreakAccelWaveInfo (Utilities|GetWave (LocalVariables|Getgrid_row) (LocalVariables|Getgrid_column))))))
    ;[1 1 1] 波の生成
    (bind _returnvalue (Game|SpawnActorfromClass "/Game/Blueprints/Field/BP_AccelWave.BP_AccelWave_C" (Math|Transform|MakeTransform (LocalVariables|Getposition) (Math|Rotator|MakeRotator 0.0 0.0 (.yaw (LocalVariables|Getrotation)))) "Undefined" 0 0))
    (bind _velocity (CallFunction|CulcVelocity (.Yaw (Math|Rotator|BreakRotator (LocalVariables|Getrotation)))))
    (Utilities|Array|SetArrayElem (Utilities|Struct|BreakAccelWaveArray (Utilities|Array|Get(acopy) (Variables|Default|GetWaveArray) (LocalVariables|Getgrid_row))) (LocalVariables|Getgrid_column) (Utilities|Struct|MakeAccelWaveInfo _velocity 7e+02 (Math|DateTime|Now) _returnvalue))))

(fn CulcGrid
  (params (Position :type Float%20%28single-precision%29) (Size :type Float%20%28single-precision%29) (Index :type Integer))
  (LocalVariables|SetNewLocalVar_0 Index)
  (if (>= (Math|Integer|Max(Integer) (Math|Integer|Min(Integer) (Math|Conversions|ToInteger(Byte) (Class|KismetMathLibrary|FCeil64 (* (LocalVariables|GetNewLocalVar_0) (/ (+ Position Size) (* 2 Size))))) (LocalVariables|GetNewLocalVar_0))) (LocalVariables|GetNewLocalVar_0))
    (return (- (Math|Integer|Max(Integer) (Math|Integer|Min(Integer) (Math|Conversions|ToInteger(Byte) (Class|KismetMathLibrary|FCeil64 (* (LocalVariables|GetNewLocalVar_0) (/ (+ Position Size) (* 2 Size))))) (LocalVariables|GetNewLocalVar_0))) 1))
    (else
      (return (Math|Integer|Max(Integer) (Math|Integer|Min(Integer) (Math|Conversions|ToInteger(Byte) (Class|KismetMathLibrary|FCeil64 (* (LocalVariables|GetNewLocalVar_0) (/ (+ Position Size) (* 2 Size))))) (LocalVariables|GetNewLocalVar_0)))))))

(fn CulcVelocity
  (params (angle :type Float%20%28single-precision%29))
  (return (Math|Vector|MakeVector (Math|Trig|Cos(Degrees) angle) (Math|Trig|Sin(Degrees) angle) 0.0)))

(fn GetAccelVelocity
  (params (position :type Vector))
  (bind _output_get (LocalVariables|SetbortPosition position))
  (bind _value (CallFunction|CulcGrid (.X (Math|Vector|BreakVector _output_get)) (Variables|Default|GetWidth) (Variables|Default|GetRow)))
  (LocalVariables|Setgrid_row _value)
  (bind _value_2 (CallFunction|CulcGrid (.Y (Math|Vector|BreakVector (LocalVariables|GetbortPosition))) (Variables|Default|GetHeight) (Variables|Default|GetColumn)))
  (LocalVariables|Setgrid_column _value_2)
  (if (Utilities|IsValid (.WaveObject (Utilities|Struct|BreakAccelWaveInfo (Utilities|GetWave (LocalVariables|Getgrid_row) (LocalVariables|Getgrid_column)))))
    (return (* (.velocity (Utilities|Struct|BreakAccelWaveInfo (Utilities|GetWave (LocalVariables|Getgrid_row) (LocalVariables|Getgrid_column)))) (.Length (Utilities|Struct|BreakAccelWaveInfo (Utilities|GetWave (LocalVariables|Getgrid_row) (LocalVariables|Getgrid_column))))))
    (else
      (return "0, 0, 0"))))