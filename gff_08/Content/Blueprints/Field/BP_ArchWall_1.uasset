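; BP_ArchWall_1 is a field arch wall Blueprint that supplies a fixed set of seventeen points.
; GetPoints returns Point1 through Point17 as an ordered array.
; The construction script only calls its parent, and the event graph holds only disabled default events, so the asset adds no runtime logic of its own.
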(event EventBeginPlay
  (|CallParentFunction) ; このノードは無効になっているため呼び出せません。\n機能をビルドするにはピンをドラッグしてください。
)

(event Collision|EventActorBeginOverlap
  (params (OtherActor :type Actor%20Object%20Reference))
  (|CallParentFunction OtherActor) ; このノードは無効になっているため呼び出せません。\n機能をビルドするにはピンをドラッグしてください。
)

(event EventTick
  (params (DeltaSeconds :type Float%20%28single-precision%29))
  (|CallParentFunction DeltaSeconds) ; このノードは無効になっているため呼び出せません。\n機能をビルドするにはピンをドラッグしてください。
)

(fn ConstructionScript
  (|CallParentFunction))

(fn GetPoints
  (return (Utilities|Array|MakeArray (Variables|Default|GetPoint1) (Variables|Default|GetPoint2) (Variables|Default|GetPoint3) (Variables|Default|GetPoint4) (Variables|Default|GetPoint5) (Variables|Default|GetPoint6) (Variables|Default|GetPoint7) (Variables|Default|GetPoint8) (Variables|Default|GetPoint9) (Variables|Default|GetPoint10) (Variables|Default|GetPoint11) (Variables|Default|GetPoint12) (Variables|Default|GetPoint13) (Variables|Default|GetPoint14) (Variables|Default|GetPoint15) (Variables|Default|GetPoint16) (Variables|Default|GetPoint17))))