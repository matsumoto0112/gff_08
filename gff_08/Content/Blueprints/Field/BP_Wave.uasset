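; BP_Wave is a field wave actor that carries a velocity and exists for a limited time after spawning.
; Initialize sets its location and rotation and stores the velocity, which GetWaveVelocity returns to callers; the graphs here never move the actor by it.
; BeginPlay records the start time, and Tick prints a debug message and destroys the actor once LimitTime seconds have elapsed.
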(event EventBeginPlay
  (Variables|Default|SetstartTime (Math|DateTime|Now)))

(event Collision|EventActorBeginOverlap
  (params (OtherActor :type Actor%20Object%20Reference)))

(event EventTick
  (params (DeltaSeconds :type Float%20%28single-precision%29))
  ;[1 1 1] 生成してからの時間を測り、時間になったら削除する
  (if (>= (Math|Timespan|GetSeconds (- (Math|DateTime|Now) (Variables|Default|GetstartTime))) (Variables|Default|GetlimitTime))
    (Development|PrintString "delete wave")
    (Actor|DestroyActor)))

(fn ConstructionScript)

(fn Initialize
  (params (Location :type Vector) (Rotation :type Rotator) (Velocity :type Vector))
  (Transformation|SetActorLocationAndRotation Location Rotation)
  (Variables|Default|Setvelocity Velocity))

(fn GetWaveVelocity
  (return (Variables|Default|Getvelocity)))