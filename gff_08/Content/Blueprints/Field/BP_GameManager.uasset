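; BP_GameManager runs a boat race from start to the switch to the result level.
; On BeginPlay it gives every BP_Boat the start checkpoint and plays music and a start sound through the game instance's sound system.
; Tick polls each boat's LapCounter, flagging race end when all finish and starting a ten-second timer, apparently to force the end, once any finishes.
; A DoOnce guards the level change.
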(event EventBeginPlay
  (Utilities|FlowControl|Sequence
    (:then_0
      (bind _outactors (Actor|GetAllActorsOfClass "/Game/Blueprints/Boat/BP_Boat.BP_Boat_C"))
      (bind _output_get (Variables|Default|SetRacingBoats _outactors))
      (for _array_element _output_get
        (Variables|/Game/Blueprints/Boat/BP_Boat.BP_Boat_C|SetNextCheckPoint _array_element (Variables|Default|GetStartCheckPoint))))
    (:then_1
      (bind _returnvalue (Class|MyGameInstance|GetInstance))
      (Utilities|IsValid _returnvalue
        (:Is%20Valid
          (Utilities|IsValid (Class|MyGameInstance|GetSoundSystem _returnvalue)
            (:Is%20Valid
              (bind _returnvalue_2 (Class|SoundSystem|PlaySound (Class|MyGameInstance|GetSoundSystem _returnvalue) "BGM_TITLE" false))
              (Variables|Default|SetBGMObject _returnvalue_2)
              (Class|SoundSystem|PlaySound (Class|MyGameInstance|GetSoundSystem _returnvalue) "SE_RACE_START" true))))))))

(event Collision|EventActorBeginOverlap
  (params (OtherActor :type Actor%20Object%20Reference)))

(event EventTick
  (params (DeltaSeconds :type Float%20%28single-precision%29))
  (Utilities|FlowControl|Sequence
    (:then_0
      (bind _raceend (CallFunction|IsRaceEnd))
      (Variables|Default|SetbIsRaceEnd (or _raceend (Variables|Default|GetbIsRaceEnd)))
      (if (not (Utilities|Time|IsValidTimerHandle (Variables|Default|GetRaceEndTimerHandle)))
        ;[1 1 1] 誰か一人でもゴールしたら一定時間後にレース終了とする
        (for _array_element (Variables|Default|GetRacingBoats)
          (if (== (Variables|/Script/gff_08.LapCounter|GetLapCount (Variables|/Game/Blueprints/Boat/BP_Boat.BP_Boat_C|GetLapCounter _array_element)) (+ (Variables|Default|GetMaxLapCount) 1))
            (bind _returnvalue (Utilities|Time|SetTimerbyEvent (EventDispatchers|CreateEvent :!event ForceRaceEnd) 1e+01))
            (Variables|Default|SetRaceEndTimerHandle _returnvalue)))))
    (:then_1
      (if (Variables|Default|GetbIsRaceEnd)
        (Utilities|FlowControl|DoOnce false
          (:Completed
            (Game|OpenLevel(byName) "result")))))))

(event EventEndPlay
  (params (EndPlayReason :type EEndPlayReason%20Enum :default "Destroyed"))
  (Actor|DestroyActor (Variables|Default|GetBGMObject)))

(fn ConstructionScript)

(fn IsRaceEnd
  (bind _goal (CallFunction|IsAllBoatGoal))
  (if _goal
    (return true)
    (else
      (return false))))

(fn IsAllBoatGoal
  (for _array_element (Variables|Default|GetRacingBoats)
    (if (not (== (Variables|/Script/gff_08.LapCounter|GetLapCount (Variables|/Game/Blueprints/Boat/BP_Boat.BP_Boat_C|GetLapCounter _array_element)) (+ (Variables|Default|GetMaxLapCount) 1)))
      (return false)))
  (return true))

(fn ForceRaceEnd
  (Variables|Default|SetbIsRaceEnd true))