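; Boat movement component that drives a physics boat mesh from a move value and left/right motor inputs.
; Forward force tapers toward max speed and stops above it, while the motor difference applies sideways force at a steering point.
; It adds push from BP_Field's wave velocity at the boat's position and runs a looping wave-spawn timer while fast enough.
; Wave-velocity deceleration is stubbed out, adding zero velocity.
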(event EventBeginPlay
  (bind _returnvalue (Actor|GetActorOfClass "/Game/Blueprints/Field/BP_Field.BP_Field_C"))
  (Variables|Default|SetField _returnvalue))

(event EventTick
  (params (DeltaSeconds :type Float%20%28single-precision%29)))

(fn Move
  (params (MoveValue :type Float%20%28single-precision%29) (LeftMotorValue :type Float%20%28single-precision%29) (RightMotorValue :type Float%20%28single-precision%29))
  (LocalVariables|SetLeftValue LeftMotorValue)
  (LocalVariables|SetRIghtValue RightMotorValue)
  (bind _isover (CallFunction|IsOverBoatMaxSpeed))
  (if _isover
    _
    (else
      (CallFunction|AddForwardForce MoveValue)))
  (CallFunction|AddRightForce (LocalVariables|GetLeftValue) (LocalVariables|GetRIghtValue))
  (CallFunction|SettingWaveGenerateTimer)
  (CallFunction|ToSpeedCentimeterPerSecond -1e+01)
  (bind _accelvelocity (Default|GetAccelVelocity (Variables|Default|GetField) (Transformation|GetActorLocation (Variables|Default|GetParentPawn))))
  ;[1 1 1] 波による加速
  (Physics|AddForce (Variables|Components|GetBoatMesh) (* (Math|Vector|Normalize _accelvelocity) 2e+06) "None" false)
  (Physics|SetPhysicsLinearVelocity (Variables|Components|GetBoatMesh) (+ (* "0, 0, 0" (Variables|Default|GetWaveDecelerationRate)) "0.000000, 0, 0") true "None"))

(fn IsOverBoatMaxSpeed
  (bind _velocitylength (CallFunction|GetBoatVelocityIgnoreWaveandOther))
  (bind _kilometerperhour (CallFunction|ToSpeedKilometerPerHour _velocitylength))
  (return (>= _kilometerperhour (Variables|Default|GetMaxSpeed))))

(fn Init
  (params (Parent :type Pawn%20Object%20Reference) (BoatMesh :type Static%20Mesh%20Component%20Object%20Reference) (SteerForceLocation :type Arrow%20Component%20Object%20Reference) (GenerateWaveLocation :type Arrow%20Component%20Object%20Reference))
  (Variables|Default|SetParentPawn Parent)
  (Variables|Components|SetBoatMesh BoatMesh)
  (Variables|Components|SetSteerForceLocation SteerForceLocation)
  (Variables|Components|SetGenerateWaveLocation GenerateWaveLocation))

(fn GetBoatVelocityIgnoreWaveandOther
  (return (Math|Vector|VectorLength (- (Transformation|GetVelocity (Variables|Default|GetParentPawn)) "0, 0, 0"))))

(fn AddForwardForce
  (params (MoveValue :type Float%20%28single-precision%29))
  (bind _boatmesh (Variables|Components|GetBoatMesh))
  (bind _velocitylength (CallFunction|GetBoatVelocityIgnoreWaveandOther))
  (bind _centimeterpersecond (CallFunction|ToSpeedCentimeterPerSecond (Variables|Default|GetMaxSpeed)))
  (Physics|AddForce _boatmesh (* (Math|Vector|GetForwardVector _boatmesh) (* MoveValue (Variables|Default|GetAcceleration) (Physics|GetMass (Variables|Components|GetBoatMesh)) (Math|Float|Lerp 1.0 0.0 (/ _velocitylength _centimeterpersecond)))) "None" false))

(fn AddRightForce
  (params (LeftMotor :type Float%20%28single-precision%29) (RightMotor :type Float%20%28single-precision%29))
  (Class|PrimitiveComponent|AddForceatLocation (Variables|Components|GetBoatMesh) (* (Math|Vector|GetRightVector (Variables|Components|GetSteerForceLocation)) (* (- LeftMotor RightMotor) (Variables|Default|GetAngularAcceleration) (Physics|GetMass (Variables|Components|GetBoatMesh)) (Math|Float|SelectFloat -1.0 1.0 (Variables|Default|GetbFlipInput)))) (Transformation|GetWorldLocation (Variables|Components|GetSteerForceLocation)) "None"))

(fn UpdateWaveVelocity
  (params (NewVelocity :type Vector)))

(fn SettingWaveGenerateTimer
  ;[1 1 1] 速度が一定値以上かどうかの判定
  (bind _kilometerperhour (CallFunction|ToSpeedKilometerPerHour (Math|Vector|VectorLength (Transformation|GetVelocity (Variables|Default|GetParentPawn)))))
  (if (>= _kilometerperhour (Variables|Default|GetWaveSpawnableSpeed))
    ;[1 1 1] 以上なら波生成タイマーを始動させる
    (if (not (Utilities|Time|IsValidTimerHandle (Variables|Default|GetCurrentWaveTimerHandle)))
      ;[1 1 1] タイマーの初期化
      (bind _returnvalue (Utilities|Time|SetTimerbyEvent (EventDispatchers|CreateEvent :!event GenerateWave) (Variables|Default|GetWaveSpawnSeconds) true))
      (Variables|Default|SetCurrentWaveTimerHandle _returnvalue))
    (else
      ;[1 1 1] 以下ならタイマーの初期化
      (Utilities|Time|ClearandInvalidateTimerbyHandle (Variables|Default|GetCurrentWaveTimerHandle)))))

(fn GenerateWave
  (bind _generatewavelocation (Variables|Components|GetGenerateWaveLocation))
  (Default|GenerateAccelWave (Variables|Default|GetField) (Transformation|GetWorldLocation _generatewavelocation) (Transformation|GetWorldRotation _generatewavelocation)))