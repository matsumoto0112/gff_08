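; Boat actor for a checkpoint-based lap race, steered through a swappable Driver that supplies left motor, right motor and back inputs.
; Mesh overlaps with checkpoints report to LapCounter and store the following checkpoint as NextCheckPoint.
; EnableAutoMode replaces the Driver with a newly constructed AIBrain for computer control.
; Each tick scales the left and right water particle rates by speed relative to BoatMover's maximum; wall-hit sound logic is left disconnected.
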(event OnComponentBeginOverlap(StaticMesh)
  (params (OverlappedComponent :type Primitive%20Component%20Object%20Reference) (OtherActor :type Actor%20Object%20Reference) (OtherComp :type Primitive%20Component%20Object%20Reference) (OtherBodyIndex :type Integer) (bFromSweep :type Boolean) (SweepResult :type Hit%20Result%20Structure%20%28by%20ref%29))
  (bind _asbp_check_point (Utilities|Casting|CastToBP_CheckPoint OtherActor))
  (Utilities|FlowControl|Sequence
    (:then_0
      (Class|LapCounter|PassCheckPoint (Variables|Default|GetLapCounter) _asbp_check_point))
    (:then_1
      (bind _asbp_check_point_2 (Utilities|Casting|CastToBP_CheckPoint (Default|GetNextPoint _asbp_check_point)))
      (Variables|Default|SetNextCheckPoint _asbp_check_point_2))))

(event OnComponentHit(StaticMesh)
  (params (HitComponent :type Primitive%20Component%20Object%20Reference) (OtherActor :type Actor%20Object%20Reference) (OtherComp :type Primitive%20Component%20Object%20Reference) (NormalImpulse :type Vector :default "0, 0, 0") (Hit :type Hit%20Result%20Structure%20%28by%20ref%29)))

(event EventBeginPlay
  (|CallParentFunction))

(event Collision|EventActorBeginOverlap
  (params (OtherActor :type Actor%20Object%20Reference)))

(event EventTick
  (params (DeltaSeconds :type Float%20%28single-precision%29))
  (|CallParentFunction DeltaSeconds)
  (|UpdateWaterParticles))

(event EventEnableAutoMode
  (bind _returnvalue (Game|ConstructObjectfromClass "/Script/gff_08.AIBrain" self))
  (Class|AIBrain|Init _returnvalue self)
  (Variables|/Script/gff_08.AIBrain|SetIntelligence _returnvalue 0.8)
  (Variables|Default|SetDriver _returnvalue))

(fn ConstructionScript)

(fn GetMotorValues
  (bind _driver (Variables|Default|GetDriver))
  (bind _returnvalue (Class|Driver|CurrentInputInfo _driver))
  (bind (_leftmotorvalue _rightmotorvalue _bback) (Utilities|Struct|BreakInputInfo _returnvalue))
  (return _leftmotorvalue _rightmotorvalue _bback))