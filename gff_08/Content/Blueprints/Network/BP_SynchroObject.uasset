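; Per-player Strix-replicated object that syncs a boat racer's identity, transform, lap events and results in multiplayer races.
; Replicated UserData spawns the boat through BP_RaceManager, whose lap counter feeds event and result data into the game instance's play data.
; Owners flag IsReady once four boats exist; the room owner counts four ready members, then sends the RaceReady RPC to start race setup.
; Input-sync logic is present but disconnected.
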(event OnSyncBegin(StrixReplicator)
  (Class|StrixBlueprintFunctionLibrary|RegisterStrixRpc 0 "RaceReady")
  (Development|PrintString "Set RPC" true true "(R=0.000000,G=0.660000,B=1.000000,A=1.000000)" 111.0))

(event EventBeginPlay
  (bind _returnvalue (Class|MyGameInstance|GetInstance))
  (bind _returnvalue_2 (Class|MyGameInstance|GetUserData _returnvalue))
  (bind _boatindex (Variables|/Script/gff_08.PlayUserData|GetBoatIndex _returnvalue_2))
  (bind _playerindex (Variables|/Script/gff_08.PlayUserData|GetPlayerIndex _returnvalue_2))
  (bind _playername (Variables|/Script/gff_08.PlayUserData|GetPlayerName _returnvalue_2))
  (bind _returnvalue_3 (Actor|GetActorOfClass "/Game/Blueprints/Stage/BP_RaceManager.BP_RaceManager_C"))
  (Variables|Default|SetRaceManager _returnvalue_3)
  (bind _returnvalue_4 (Class|NetworkConnectUtility|IsMultiGame))
  (if _returnvalue_4
    (bind _returnvalue_5 (Class|NetworkConnectUtility|IsOwner self))
    (if _returnvalue_5
      (Variables|Default|SetUserData (Utilities|Struct|MakeNetworkUserData _playerindex _playername _boatindex))
      (Class|StrixBlueprintFunctionLibrary|UnpauseNetworkObjectManager (Variables|/Script/gff_08.PlayUserData|GetChannelID _returnvalue_2))
      (Utilities|Time|SetTimerbyEvent (EventDispatchers|CreateEvent :!event UpdateLocationandRotation) 1.0 true)
      (Development|PrintText (Utilities|Text|FormatText "PlayerID:{0} BoatID:{1} Name:{2}" _playerindex _boatindex _playername))
      (bind _returnvalue_6 (Utilities|Time|SetTimerbyEvent (EventDispatchers|CreateEvent :!event CheckOwnerRaceReady) 1.0 true))
      (Variables|Default|SetOwnerHandle _returnvalue_6)
      (bind _returnvalue_7 (Class|StrixBlueprintFunctionLibrary|IsRoomOwner (Variables|/Script/gff_08.NetworkData|GetChannelID (Class|MyGameInstance|GetNetworkData (Class|MyGameInstance|GetInstance)))))
      (if _returnvalue_7
        (bind _returnvalue_8 (Utilities|Time|SetTimerbyEvent (EventDispatchers|CreateEvent :!event CheckRoomOwnerRaceReady) 1.0 true))
        (Variables|Default|SetRoomOwnerHandle _returnvalue_8)))))

(event Collision|EventActorBeginOverlap
  (params (OtherActor :type Actor%20Object%20Reference)))

(event EventTick
  (params (DeltaSeconds :type Float%20%28single-precision%29))
  (bind _returnvalue (Class|NetworkConnectUtility|IsOwner self))
  (if _returnvalue
    _))

(event EventEndPlay
  (params (EndPlayReason :type EEndPlayReason%20Enum :default "Destroyed")))

(fn ConstructionScript)

(fn OnRepUserData
  (if (not (Variables|Default|GetbCalledFirstReplecated_UserData))
    (if (!= (.playerindex (Variables|Default|GetUserData)) -1)
      (Actor|GetActorOfClass "/Game/Blueprints/Stage/BP_RaceManager.BP_RaceManager_C")
      (bind _returnvalue (Class|RaceManager|SpawnBoat (Variables|Default|GetRaceManager) (Variables|Default|GetUserData)))
      (bind _output_get (Variables|Default|SetMyBoat _returnvalue))
      (EventDispatchers|BindEventtoLapIncrementDispatcher (Variables|/Script/gff_08.Boat|GetLapCounter _output_get) (EventDispatchers|CreateEvent :!event LapIncrementEvent))
      (Variables|Default|SetbCalledFirstReplecated_UserData true) ; 複数回呼ばれるのを防止する
    )))

(fn UpdateLocationandRotation
  (bind _myboat (Variables|Default|GetMyBoat))
  (bind _returnvalue (Transformation|GetActorTransform _myboat))
  (bind _returnvalue_2 (Class|NetworkConnectUtility|IsOwner self))
  (if _returnvalue_2
    (Variables|Default|SetTransformData (Utilities|Struct|MakeNetworkTransformData (.location _returnvalue) (.rotation _returnvalue)))
    (else
      (Transformation|SetActorLocationAndRotation (Variables|Default|GetMyBoat) (.fixlocation (Variables|Default|GetTransformData)) (.fixrotation (Variables|Default|GetTransformData))))))

(fn OnRepEventData)

(fn LapIncrementEvent
  (params (NextLapCount :type Integer))
  (bind _myboat (Variables|Default|GetMyBoat))
  (bind _lapcounter (Variables|/Script/gff_08.Boat|GetLapCounter _myboat))
  (bind _returnvalue (Class|LapCounter|GetLapTimes _lapcounter))
  (Development|PrintText (Utilities|Text|FormatText "{0} Lap is {1}" (.playername (Variables|Default|GetUserData)) NextLapCount))
  (switch int NextLapCount
    (:2
      (Variables|Default|SetEventData (Utilities|Struct|MakeNetworkEventData "LAP_1" "0001.01.01-00.00.00")))
    (:3
      (Variables|Default|SetEventData (Utilities|Struct|MakeNetworkEventData "LAP_2" "0001.01.01-00.00.00")))
    (:4
      (Variables|Default|SetEventData (Utilities|Struct|MakeNetworkEventData "GOAL" "0001.01.01-00.00.00"))
      (Variables|Default|SetResultData (Utilities|Struct|MakeNetworkResultData (Utilities|Array|Get(acopy) _returnvalue) (Utilities|Array|Get(acopy) _returnvalue 1) (Utilities|Array|Get(acopy) _returnvalue 2))))))

(fn OnRepResultData
  (bind _returnvalue (Class|MyGameInstance|GetInstance))
  (bind _userdata (Variables|Default|GetUserData))
  (bind _resultdata (Variables|Default|GetResultData))
  (bind _returnvalue_2 (Class|MyGameInstance|GetPlayData _returnvalue))
  (Utilities|Array|SetArrayElem (.allracersdata _returnvalue_2) (.playerindex _userdata) (Utilities|Struct|MakeGamePlayData -1 (.playername _userdata) (Utilities|Array|MakeArray (.confirmlaptime_1 _resultdata) (.confirmlaptime_2 _resultdata) (.confirmlaptime_3 _resultdata))))
  (Class|MyGameInstance|SetPlayData _returnvalue (Utilities|Struct|MakeAllRacersGamePlayData (.myboatindex _returnvalue_2) 0)))

(fn CheckOwnerRaceReady
  (bind _returnvalue (Class|MyGameInstance|GetInstance))
  (bind _returnvalue_2 (Class|MyGameInstance|GetNetworkData _returnvalue))
  (if (Class|StrixReplicatorComponent|GetIsOwner (Variables|Default|GetStrixReplicator))
    (Actor|GetActorOfClass "/Game/Blueprints/Stage/BP_RaceManager.BP_RaceManager_C")
    (if (== (Utilities|Array|Length (Variables|/Script/gff_08.RaceManager|GetBoats (Variables|Default|GetRaceManager))) 4)
      (Class|StrixBlueprintFunctionLibrary|SetRoomMember (Variables|/Script/gff_08.NetworkData|GetChannelID _returnvalue_2) (Class|NetworkData|SetBoolMemberProperty _returnvalue_2 "IsReady" true))
      (Utilities|Time|PauseTimerbyHandle (Variables|Default|GetOwnerHandle))
      (Development|PrintString "OK,SetUp" true true "(R=0.000000,G=0.047143,B=1.000000,A=1.000000)" 111.0))))

(fn RaceReady
  (Development|PrintString "Call RPC Method" true true "(R=0.000000,G=0.660000,B=1.000000,A=1.000000)" 111.0)
  (Development|PrintString "PlayStart!!!!!" true true "(R=1.000000,G=0.115352,B=0.000000,A=1.000000)" 111.0)
  (bind _returnvalue (Actor|GetActorOfClass "/Game/Blueprints/Stage/BP_RaceManager.BP_RaceManager_C"))
  (Class|RaceManager|StartRaceSetUp _returnvalue))

(fn CheckRoomOwnerRaceReady
  (LocalVariables|SetCount 0)
  (bind _returnvalue (Class|StrixBlueprintFunctionLibrary|GetCurrentRoomMembers (Variables|/Script/gff_08.NetworkData|GetChannelID (Class|MyGameInstance|GetNetworkData (Class|MyGameInstance|GetInstance)))))
  (for _array_element _returnvalue
    (if (.result (Class|StrixBlueprintFunctionLibrary|TryGetBoolProperty (.properties _array_element) "IsReady"))
      (if (.value (Class|StrixBlueprintFunctionLibrary|TryGetBoolProperty (.properties _array_element) "IsReady"))
        (LocalVariables|SetCount (+ (LocalVariables|GetCount) 1)))))
  (if (== (LocalVariables|GetCount) 4)
    (Development|PrintString "Send RPC to other members" true true "(R=1.000000,G=0.107360,B=0.000000,A=1.000000)" 111.0)
    (Utilities|Time|PauseTimerbyHandle (Variables|Default|GetRoomOwnerHandle))
    (Class|StrixBlueprintFunctionLibrary|SendRpctoAll 0 "RaceReady")
    (Class|StrixBlueprintFunctionLibrary|SendRpctoOtherMembers 0 "RaceReady")
    (Development|PrintString "Hello")
    (else
      (Development|PrintString "Please Wait..." true true "(R=1.000000,G=0.022841,B=0.000000,A=1.000000)" 112.0))))

(fn OnRepTransformData
  (CallFunction|UpdateLocationandRotation))