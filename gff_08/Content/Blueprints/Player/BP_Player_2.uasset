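; Player pawn for a physics-driven craft steered by two motor axes, riding and spawning waves on a BP_Field.
; The shared motor input drives capped forward force, while the left/right difference applies steering force at an offset point.
; Each tick it adjusts velocity using current and scaled previous wave velocity, currently fed a constant test wave.
; Above a speed threshold, a looping timer runs for spawning acceleration waves on the field.
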(event EventBeginPlay
  (bind _returnvalue (Actor|GetActorOfClass "/Game/Blueprints/Field/BP_Field.BP_Field_C"))
  (Variables|Default|SetField _returnvalue))

(event Collision|EventActorBeginOverlap
  (params (OtherActor :type Actor%20Object%20Reference)))

(event EventTick
  (params (DeltaSeconds :type Float%20%28single-precision%29))
  (CallFunction|Movement)
  (CallFunction|SettingWaveGenerateTimer)
  ;[1 1 1] 波のテスト　10km/hの速度で-y方向に動く
  (bind _centimeterpersecond (CallFunction|ToSpeedCentimeterPerSecond -1e+01))
  (CallFunction|UpdateWave (Math|Vector|MakeVector _centimeterpersecond _centimeterpersecond 0.0)))

(event Input|ActionEvents|InputActionExitGame
  (params (Key :type Key%20Structure :default "None"))
  (:Pressed
    (Game|QuitGame 0 "Quit" false)))

(event Input|AxisEvents|InputAxisLeft_Motor
  (params (AxisValue :type Float%20%28single-precision%29))
  (Variables|Default|SetLeftMotorValue AxisValue))

(event Input|AxisEvents|InputAxisRight_Motor
  (params (AxisValue :type Float%20%28single-precision%29))
  (Variables|Default|SetRightMotorValue AxisValue))

(fn ConstructionScript)

(fn CalcMovementValues
  (bind _leftmotorvalue (Variables|Default|GetLeftMotorValue))
  (bind _rightmotorvalue (Variables|Default|GetRightMotorValue))
  (bind _returnvalue (Math|Float|Min(Float) _leftmotorvalue _rightmotorvalue))
  (return _returnvalue (- (Variables|Default|GetLeftMotorValue) _returnvalue) (- (Variables|Default|GetRightMotorValue) _returnvalue)))

(fn GetPlayerSpeed
  (bind _kilometerperhour (CallFunction|ToSpeedKilometerPerHour (Math|Vector|VectorLength (Transformation|GetVelocity))))
  (return _kilometerperhour))

(fn Movement
  (bind (_movevalue _leftvalue _rightvalue) (CallFunction|CalcMovementValues)) ; 移動量と回転量を計算する
  (LocalVariables|SetMoveValue _movevalue)
  (LocalVariables|SetLeftValue _leftvalue)
  (LocalVariables|SetRightValue _rightvalue)
  ;[1 1 1] 最高速度を超えているか
  (bind _kilometerperhour (CallFunction|ToSpeedKilometerPerHour (Math|Vector|VectorLength (- (Transformation|GetVelocity) (Variables|Default|GetPrevWaveVelocity)))))
  (if (>= _kilometerperhour (Variables|Default|GetMaxSpeed))
    _
    (else
      (CallFunction|AddForwardForce (LocalVariables|GetMoveValue))))
  (CallFunction|AddRightForce (LocalVariables|GetLeftValue) (LocalVariables|GetRightValue))
  ;[1 1 1] 波による加速
  (Physics|SetPhysicsLinearVelocity (Variables|Default|GetStaticMesh) (+ (* (Variables|Default|GetPrevWaveVelocity) (Variables|Default|GetWaveDecelerationRate)) (Variables|Default|GetWaveVelocity)) true "None"))

(fn AddForwardForce
  (params (MoveValue :type Float%20%28single-precision%29))
  (bind _staticmesh (Variables|Default|GetStaticMesh))
  (Physics|AddForce _staticmesh (* (Math|Vector|GetForwardVector _staticmesh) (* MoveValue (Variables|Default|GetAcceleration) (Physics|GetMass (Variables|Default|GetStaticMesh)))) "None" false))

(fn AddRightForce
  (params (LeftValue :type Float%20%28single-precision%29) (RightValue :type Float%20%28single-precision%29))
  (Class|PrimitiveComponent|AddForceatLocation (Variables|Default|GetStaticMesh) (* (Math|Vector|GetRightVector (Variables|Default|GetSteerForceLocation)) (* (- LeftValue RightValue) (Variables|Default|GetAngularAcceleration) (Physics|GetMass (Variables|Default|GetStaticMesh)) (Math|Float|SelectFloat -1.0 1.0 (Variables|Default|GetbFlipInput)))) (Transformation|GetWorldLocation (Variables|Default|GetSteerForceLocation)) "None"))

(fn GetMotorValues
  (return (Variables|Default|GetLeftMotorValue) (Variables|Default|GetRightMotorValue)))

(fn GenerateWave
  (Default|GenerateAccelWave (Variables|Default|GetField) (Transformation|GetActorTransform)))

(fn SettingWaveGenerateTimer
  ;[1 1 1] 速度が一定値以上かどうかの判定
  (bind _kilometerperhour (CallFunction|ToSpeedKilometerPerHour (Math|Vector|VectorLength (Transformation|GetVelocity))))
  (if (>= _kilometerperhour (Variables|Default|GetWaveSpawnableSpeed))
    ;[1 1 1] 以上なら波生成タイマーを始動させる
    (if (not (Utilities|Time|IsValidTimerHandle (Variables|Default|GetCurrentTimerHandle)))
      ;[1 1 1] タイマーの初期化
      (bind _returnvalue (Utilities|Time|SetTimerbyEvent (EventDispatchers|CreateEvent :!event GenerateWave) (Variables|Default|GetWaveSpawnTime) true))
      (Variables|Default|SetCurrentTimerHandle _returnvalue))
    (else
      ;[1 1 1] 以下ならタイマーの初期化
      (Utilities|Time|ClearandInvalidateTimerbyHandle (Variables|Default|GetCurrentTimerHandle)))))

(fn UpdateWave
  (params (NextWaveVelocity :type Vector))
  (Variables|Default|SetPrevWaveVelocity (Variables|Default|GetWaveVelocity))
  (Variables|Default|SetWaveVelocity NextWaveVelocity))