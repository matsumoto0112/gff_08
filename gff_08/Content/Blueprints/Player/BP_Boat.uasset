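; BP_Boat is the player's boat, driven by separate left and right motor values.
; Each tick it splits them into shared forward thrust (the minimum) and per-side surplus, then passes these to BPBoatMover.
; BPBoatMover is initialized with the mesh and a steering force location.
; It also caches the BP_Field actor, exposes motor values and speed in km/h, and quits the game on ExitGame input.
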(event EventBeginPlay
  (bind _returnvalue (Actor|GetActorOfClass "/Game/Blueprints/Field/BP_Field.BP_Field_C"))
  (Variables|Default|SetField _returnvalue)
  (Default|Init (Variables|Default|GetBP_BoatMover) self (Variables|Default|GetStaticMesh) (Variables|Default|GetSteerForceLocation)))

(event Collision|EventActorBeginOverlap
  (params (OtherActor :type Actor%20Object%20Reference)))

(event EventTick
  (params (DeltaSeconds :type Float%20%28single-precision%29))
  (bind (_movevalue _leftvalue _rightvalue) (CallFunction|CalcMovementValues))
  (Default|Move (Variables|Default|GetBP_BoatMover) _movevalue _leftvalue _rightvalue))

(event Input|ActionEvents|InputActionExitGame
  (params (Key :type Key%20Structure :default "None"))
  (:Pressed
    (Game|QuitGame 0 "Quit" false)))

(fn ConstructionScript)

(fn CalcMovementValues
  (bind _leftmotorvalue (Variables|Default|GetLeftMotorValue))
  (bind _rightmotorvalue (Variables|Default|GetRightMotorValue))
  (bind _returnvalue (Math|Float|Min(Float) _leftmotorvalue _rightmotorvalue))
  (return _returnvalue (- (Variables|Default|GetLeftMotorValue) _returnvalue) (- (Variables|Default|GetRightMotorValue) _returnvalue)))

(fn GetPlayerSpeed
  (bind _kilometerperhour (CallFunction|ToSpeedKilometerPerHour (Math|Vector|VectorLength (Transformation|GetVelocity))))
  (return _kilometerperhour))

(fn GetMotorValues
  (return (Variables|Default|GetLeftMotorValue) (Variables|Default|GetRightMotorValue)))