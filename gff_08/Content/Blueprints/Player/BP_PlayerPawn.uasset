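; Player pawn driven by two motor axis inputs in a differential, tank-like scheme, with speed settings converted to cm/s units on BeginPlay.
; Each tick, the lower motor value becomes forward movement input, while the difference between motors feeds a yaw velocity for the RotatingMovement component.
; Yaw velocity accumulates with 0.9 per-tick damping independent of delta time and is printed for debugging.
; GetPlayerSpeed reports current speed in km/h.
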(event EventBeginPlay
  (bind _centimeterpersecond (CallFunction|ToSpeedCentimeterPerSecond (Variables|Default|GetMaxMoveSpeed)))
  (Variables|/Script/Engine.FloatingPawnMovement|SetMaxSpeed (Variables|Default|GetMovementComponent) _centimeterpersecond)
  (bind _centimeterpersecond_2 (CallFunction|ToSpeedCentimeterPerSecond (Variables|Default|GetAcceleration)))
  (Variables|/Script/Engine.FloatingPawnMovement|SetAcceleration (Variables|Default|GetMovementComponent) _centimeterpersecond_2)
  (bind _centimeterpersecond_3 (CallFunction|ToSpeedCentimeterPerSecond (Variables|Default|GetDeceleration)))
  (Variables|/Script/Engine.FloatingPawnMovement|SetDeceleration (Variables|Default|GetMovementComponent) _centimeterpersecond_3))

(event Collision|EventActorBeginOverlap
  (params (OtherActor :type Actor%20Object%20Reference)))

(event EventTick
  (params (DeltaSeconds :type Float%20%28single-precision%29))
  (bind _leftmotorvalue (Variables|Default|GetLeftMotorValue))
  (bind _rightmotorvalue (Variables|Default|GetRightMotorValue))
  (bind _returnvalue (Math|Float|Min(Float) _leftmotorvalue _rightmotorvalue))
  (CallFunction|Move _returnvalue)
  (CallFunction|Rotate (- (Variables|Default|GetLeftMotorValue) _returnvalue) (- (Variables|Default|GetRightMotorValue) _returnvalue)))

(event Input|AxisEvents|InputAxisLeft_Motor
  (params (AxisValue :type Float%20%28single-precision%29))
  (Variables|Default|SetLeftMotorValue AxisValue))

(event Input|AxisEvents|InputAxisRight_Motor
  (params (AxisValue :type Float%20%28single-precision%29))
  (Variables|Default|SetRightMotorValue AxisValue))

(fn ConstructionScript)

(fn Move
  (params (MoveValue :type Float%20%28single-precision%29))
  (Pawn|Input|AddMovementInput (Transformation|GetActorForwardVector) MoveValue false))

(fn Rotate
  (params (LeftMotorValue :type Float%20%28single-precision%29) (RightMotorValue :type Float%20%28single-precision%29))
  (bind _output_get (Variables|Default|SetAngularVelocity (+ (Variables|Default|GetAngularVelocity) (* (- LeftMotorValue RightMotorValue) (Variables|Default|GetRotateSpeed)))))
  (bind _output_get_2 (Variables|/Script/Engine.RotatingMovementComponent|SetRotationRate (Variables|Default|GetRotatingMovement) (Math|Rotator|MakeRotator 0.0 0.0 _output_get)))
  (Variables|Default|SetAngularVelocity (* (Variables|Default|GetAngularVelocity) 0.9))
  (Development|PrintString (Utilities|String|ToString(Float) (.Yaw (Math|Rotator|BreakRotator _output_get_2)))))

(fn GetPlayerSpeed
  (bind _kilometerperhour (CallFunction|ToSpeedKilometerPerHour (Math|Vector|VectorLength (Transformation|GetVelocity))))
  (return _kilometerperhour))