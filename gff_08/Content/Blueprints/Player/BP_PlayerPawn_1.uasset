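; BP_PlayerPawn_1 is a player pawn driven along its forward vector by two motor input axes.
; The Left_Motor and Right_Motor axis events store their values, and Tick passes the smaller one to Move, which applies it as movement input.
; The difference between the motors is not used, so this graph does no turning.
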(event EventBeginPlay)

(event Collision|EventActorBeginOverlap
  (params (OtherActor :type Actor%20Object%20Reference)))

(event EventTick
  (params (DeltaSeconds :type Float%20%28single-precision%29))
  (CallFunction|Move (Math|Float|Min(Float) (Variables|Default|GetLeftMotorValue) (Variables|Default|GetRightMotorValue))))

(event Input|AxisEvents|InputAxisLeft_Motor
  (params (AxisValue :type Float%20%28single-precision%29))
  (Variables|Default|SetLeftMotorValue AxisValue))

(event Input|AxisEvents|InputAxisRight_Motor
  (params (AxisValue :type Float%20%28single-precision%29))
  (Variables|Default|SetRightMotorValue AxisValue))

(fn ConstructionScript)

(fn Move
  (params (MoveValue :type Float%20%28single-precision%29))
  (bind _output_get (LocalVariables|SetValue MoveValue))
  (Pawn|Input|AddMovementInput (Transformation|GetActorForwardVector) _output_get false))