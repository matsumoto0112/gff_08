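; Replicated player Blueprint for a boat race, extending a parent class and setting itself as Driver on BeginPlay.
; A temporary boat-restore input action returns the player to the previous checkpoint.
; Start looks up BP_RaceManager in the level and triggers its race setup.
; CurrentInputInfo exposes the stored InputInfo, while Tick and the construction script only call the parent.
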(event Collision|EventActorBeginOverlap
  (params (OtherActor :type Actor%20Object%20Reference))
  (|CallParentFunction OtherActor) ; This node is disabled and will not be called.\nDrag off pins to build functionality.
)

(event EventTick
  (params (DeltaSeconds :type Float%20%28single-precision%29))
  (|CallParentFunction DeltaSeconds))

(event EventBeginPlay
  (Variables|Default|SetDriver self)
  (|CallParentFunction))

(event Input|ActionEvents|InputActionBoatRotateRestore_Temp
  (params (Key :type Key%20Structure :default "None"))
  (:Pressed
    (Class|Boat|ReturnPrevCheckPoint)))

(fn ConstructionScript
  (|CallParentFunction))

(fn Start
  (bind _returnvalue (Actor|GetActorOfClass "/Game/Blueprints/Stage/BP_RaceManager.BP_RaceManager_C"))
  (Class|RaceManager|StartRaceSetUp _returnvalue))

(fn CurrentInputInfo
  (return (Variables|Default|GetInputInfo)))