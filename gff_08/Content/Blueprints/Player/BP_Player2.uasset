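; Player Blueprint that drives like a twin-motor vehicle, steered by separate left and right motor input axes.
; Each tick, the lower motor value becomes forward thrust along yaw, while the remaining difference adds yaw spin.
; Velocity and spin accumulate and decay by fixed per-frame damping, applied through swept world offset and rotation.
; Helpers convert speed to km/h for reporting and for limiting velocity once it reaches MaxMoveSpeed.
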(event EventBeginPlay)

(event Collision|EventActorBeginOverlap
  (params (OtherActor :type Actor%20Object%20Reference)))

(event EventTick
  (params (DeltaSeconds :type Float%20%28single-precision%29))
  (bind (_movevalue _leftmotorvalue _rightmotorvalue) (CallFunction|CalcMoveandRotateValues))
  (CallFunction|Move _movevalue)
  (CallFunction|Rotate _leftmotorvalue _rightmotorvalue))

(event Input|AxisEvents|InputAxisLeft_Motor
  (params (AxisValue :type Float%20%28single-precision%29))
  (Variables|Default|SetLeftMotorValue AxisValue))

(event Input|AxisEvents|InputAxisRight_Motor
  (params (AxisValue :type Float%20%28single-precision%29))
  (Variables|Default|SetRightMotorValue AxisValue))

(fn ConstructionScript)

(fn Move
  (params (MoveValue :type Float%20%28single-precision%29))
  (bind _returnvalue (Transformation|GetActorRotation))
  (bind _yaw (Math|Rotator|BreakRotator _returnvalue))
  (LocalVariables|SetValue MoveValue)
  (Variables|Default|SetVelocity (+ (Variables|Default|GetVelocity) (Math|Vector|MakeVector (* (LocalVariables|GetValue) (Math|Trig|Cos(Degrees) _yaw)) (* (Math|Trig|Sin(Degrees) _yaw) (LocalVariables|GetValue)) 0.0)))
  ;[1 1 1] 移動処理
  (CallFunction|LimitVelocity)
  (bind _sweephitresult (Transformation|AddActorWorldOffset (* (Variables|Default|GetVelocity) (* (Utilities|Time|GetWorldDeltaSeconds) (Variables|Default|GetMoveSpeed))) true))
  (Development|PrintString (Utilities|String|ToString(Boolean) (.bBlockingHit (Collision|BreakHitResult _sweephitresult))))
  ;[1 1 1] 減速処理
  (Variables|Default|SetVelocity (* (Variables|Default|GetVelocity) 0.99)))

(fn Rotate
  (params (LeftValue :type Float%20%28single-precision%29) (RightValue :type Float%20%28single-precision%29))
  (bind _output_get (Variables|Default|SetAngularVelocity (+ (Variables|Default|GetAngularVelocity) (* (- LeftValue (* RightValue 1.0)) (Variables|Default|GetRotateSpeed)))))
  (Class|Actor|AddActorWorldRotation (Math|Vector|RotatorfromAxisandAngle "0, 0,1.000000" _output_get) true)
  (Variables|Default|SetAngularVelocity (* (Variables|Default|GetAngularVelocity) 0.9)))

(fn CalcMoveandRotateValues
  (bind _leftmotorvalue (Variables|Default|GetLeftMotorValue))
  (bind _rightmotorvalue (Variables|Default|GetRightMotorValue))
  (bind _returnvalue (Math|Float|Min(Float) _leftmotorvalue _rightmotorvalue))
  (return _returnvalue (- (Variables|Default|GetLeftMotorValue) _returnvalue) (- (Variables|Default|GetRightMotorValue) _returnvalue)))

(fn GetPlayerVelocity
  (return (* (Math|Vector|VectorLength (* (Variables|Default|GetVelocity) (Variables|Default|GetMoveSpeed))) 0.036)))

(fn LimitVelocity
  (bind _over (CallFunction|IsOverMaxSpeed))
  (if _over
    ;[1 1 1] 最高速度より小さくさせる
    (Variables|Default|SetVelocity (/ (Variables|Default|GetVelocity) (/ (/ (* (Math|Vector|VectorLength (Variables|Default|GetVelocity)) (Variables|Default|GetMoveSpeed)) (/ (Variables|Default|GetRightMotorValue) 0.036)) (Variables|Default|GetMaxMoveSpeed))))))

(fn IsOverMaxSpeed
  (bind _speedperhour (CallFunction|ConverttoPerHour (Variables|Default|GetVelocity) (Variables|Default|GetMoveSpeed)))
  (return (>= _speedperhour (Variables|Default|GetMaxMoveSpeed))))

(fn ConverttoPerHour
  (params (Velocity :type Vector) (Speed :type Float%20%28single-precision%29))
  (return (* (Math|Vector|VectorLength (* Velocity Speed)) 0.036)))

(fn ConverttoPerSecond
  (params (Velocity :type Vector) (Speed :type Float%20%28single-precision%29))
  (return (/ (Math|Vector|VectorLength (* Velocity Speed)) 0.036)))