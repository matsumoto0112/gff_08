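; BP_BoatMover drives a physics-based player boat, applying thrust and steering to the mesh supplied through Init.
; Move adds mass-scaled forward force below max speed, measured without wave velocity, and steers by the left/right motor difference at an offset point.
; It also adds a currently fixed wave velocity plus the previous one scaled by a tuned deceleration rate.
; Above a speed threshold, a looping timer is set for spawning acceleration waves through BP_Field.
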(event EventBeginPlay
  (bind _returnvalue (Actor|GetActorOfClass "/Game/Blueprints/Field/BP_Field.BP_Field_C"))
  (Variables|Default|SetField _returnvalue))

(event EventTick
  (params (DeltaSeconds :type Float%20%28single-precision%29)))

(fn Move
  (params (MoveValue :type Float%20%28single-precision%29) (LeftMotorValue :type Float%20%28single-precision%29) (RightMotorValue :type Float%20%28single-precision%29))
  (LocalVariables|SetLeftValue LeftMotorValue)
  (LocalVariables|SetRIghtValue RightMotorValue)
  (bind _isover (CallFunction|IsOverBoatMaxSpeed))
  (if _isover
    _
    (else
      (CallFunction|AddForwardForce MoveValue)))
  (CallFunction|AddRightForce (LocalVariables|GetLeftValue) (LocalVariables|GetRIghtValue))
  (CallFunction|SettingWaveGenerateTimer)
  (bind _centimeterpersecond (CallFunction|ToSpeedCentimeterPerSecond -1e+01))
  ;[1 1 1] 波による加速
  (CallFunction|UpdateWaveVelocity (Math|Vector|MakeVector _centimeterpersecond _centimeterpersecond 0.0))
  (Physics|SetPhysicsLinearVelocity (Variables|Default|GetBoatMesh) (+ (* (Variables|Default|GetPrevWaveVelociry) (Variables|Default|GetWaveDecelerationRate)) (Variables|Default|GetWaveVelocity)) true "None"))

(fn IsOverBoatMaxSpeed
  (bind _velocitylength (CallFunction|GetBoatVelocityIgnoreWaveandOther))
  (bind _kilometerperhour (CallFunction|ToSpeedKilometerPerHour _velocitylength))
  (return (>= _kilometerperhour (Variables|Default|GetMaxSpeed))))

(fn Init
  (params (Parent :type Pawn%20Object%20Reference) (BoatMesh :type Static%20Mesh%20Component%20Object%20Reference) (SteerForceLocation :type Arrow%20Component%20Object%20Reference))
  (Variables|Default|SetParentPawn Parent)
  (Variables|Default|SetBoatMesh BoatMesh)
  (Variables|Default|SetSteerForceLocation SteerForceLocation))

(fn GetBoatVelocityIgnoreWaveandOther
  (return (Math|Vector|VectorLength (- (Transformation|GetVelocity (Variables|Default|GetParentPawn)) (Variables|Default|GetPrevWaveVelociry)))))

(fn AddForwardForce
  (params (MoveValue :type Float%20%28single-precision%29))
  (bind _boatmesh (Variables|Default|GetBoatMesh))
  (Physics|AddForce _boatmesh (* (Math|Vector|GetForwardVector _boatmesh) (* MoveValue (Variables|Default|GetAcceleration) (Physics|GetMass (Variables|Default|GetBoatMesh)))) "None" false))

(fn AddRightForce
  (params (LeftMotor :type Float%20%28single-precision%29) (RightMotor :type Float%20%28single-precision%29))
  (Class|PrimitiveComponent|AddForceatLocation (Variables|Default|GetBoatMesh) (* (Math|Vector|GetRightVector (Variables|Default|GetSteerForceLocation)) (* (- LeftMotor RightMotor) (Variables|Default|GetAngularAcceleration) (Physics|GetMass (Variables|Default|GetBoatMesh)) (Math|Float|SelectFloat -1.0 1.0 (Variables|Default|GetbFlipInput)))) (Transformation|GetWorldLocation (Variables|Default|GetSteerForceLocation)) "None"))

(fn UpdateWaveVelocity
  (params (NewVelocity :type Vector))
  (Variables|Default|SetPrevWaveVelociry (Variables|Default|GetWaveVelocity))
  (Variables|Default|SetWaveVelocity NewVelocity))

(fn SettingWaveGenerateTimer
  ;[1 1 1] 速度が一定値以上かどうかの判定
  (bind _kilometerperhour (CallFunction|ToSpeedKilometerPerHour (Math|Vector|VectorLength (Transformation|GetVelocity (Variables|Default|GetParentPawn)))))
  (if (>= _kilometerperhour (Variables|Default|GetWaveSpawnableSpeed))
    ;[1 1 1] 以上なら波生成タイマーを始動させる
    (if (not (Utilities|Time|IsValidTimerHandle (Variables|Default|GetCurrentWaveTimerHandle)))
      ;[1 1 1] タイマーの初期化
      (bind _returnvalue (Utilities|Time|SetTimerbyEvent (EventDispatchers|CreateEvent :!event GenerateWave) (Variables|Default|GetWaveSpawnSeconds) true))
      (Variables|Default|SetCurrentWaveTimerHandle _returnvalue))
    (else
      ;[1 1 1] 以下ならタイマーの初期化
      (Utilities|Time|ClearandInvalidateTimerbyHandle (Variables|Default|GetCurrentWaveTimerHandle)))))

(fn GenerateWave
  (Default|GenerateAccelWave (Variables|Default|GetField) (Transformation|GetActorTransform (Variables|Default|GetParentPawn))))