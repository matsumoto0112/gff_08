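; BP_Player is the player-driven boat in a race, setting itself as Driver and packaging left/right motor values and Back input as input info.
; Each tick it drives concentration and water-drop post-process parameters in MPC_PostProcess from the boat's acceleration field, with a gradual fade.
; Input events also handle quitting, auto mode, checkpoint return and a test race-end call, while Start triggers BP_RaceManager's race setup.
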(event Collision|EventActorBeginOverlap
  (params (OtherActor :type Actor%20Object%20Reference))
  (|CallParentFunction OtherActor) ; This node is disabled and will not be called.\nDrag off pins to build functionality.
)

(event EventTick
  (params (DeltaSeconds :type Float%20%28single-precision%29))
  (|CallParentFunction DeltaSeconds)
  (|UpdateConcentraitPostProcessParameter))

(event EventBeginPlay
  (Variables|Default|SetDriver self)
  (|CallParentFunction))

(event Input|ActionEvents|InputActionExitGame
  (params (Key :type Key%20Structure :default "None"))
  (:Pressed
    (Game|QuitGame 0 "Quit" false)))

(event Input|ActionEvents|InputActionBack
  (params (Key :type Key%20Structure :default "None"))
  (:Pressed
    (Variables|Default|SetbInputBackButton true))
  (:Released
    (Variables|Default|SetbInputBackButton false)))

(event Input|ActionEvents|InputActionBoatRotateRestore_Temp
  (params (Key :type Key%20Structure :default "None"))
  (:Pressed
    (Class|Boat|ReturnPrevCheckPoint)))

(event Input|KeyboardEvents|RightShift
  (params (Key :type Key%20Structure :default "None"))
  (:Pressed
    (bind _returnvalue (Actor|GetActorOfClass "/Game/Blueprints/Stage/BP_RaceManager.BP_RaceManager_C"))
    (Development|PrintString "CallTest RaceEndEvent")
    (Class|RaceManager|TestCallRaceEndEventFunction _returnvalue)))

(event Input|KeyboardEvents|LeftBracket
  (params (Key :type Key%20Structure :default "None"))
  (:Pressed
    (CallFunction|EnableAutoMode)))

(fn ConstructionScript
  (|CallParentFunction))

(fn Start
  (bind _returnvalue (Actor|GetActorOfClass "/Game/Blueprints/Stage/BP_RaceManager.BP_RaceManager_C"))
  (Class|RaceManager|StartRaceSetUp _returnvalue))

(fn CurrentInputInfo
  (return (Utilities|Struct|MakeInputInfo (Input|AxisValues|GetLeft_Motor) (Input|AxisValues|GetRight_Motor) (Variables|Default|GetbInputBackButton))))