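; Camera director for capturing race video, switching between per-boat follow cameras and fixed-point cameras.
; When EnableVideo is off, BeginPlay destroys all BP_FixedPointCamera actors and itself.
; Tick waits until BP_RaceManager has four boats, then once spawns a BP_Stalker targeting each, appends the fixed-point cameras and enables the default camera.
; Number pad keys enable cameras by array index.
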(event EventBeginPlay
  (if (not (Variables|Default|GetbEnableVideo))
    (bind _outactors (Actor|GetAllActorsOfClass "/Game/Blueprints/Camera/BP_FixedPointCamera.BP_FixedPointCamera_C"))
    (for _array_element _outactors
      (Actor|DestroyActor _array_element))
    (Actor|DestroyActor)))

(event Collision|EventActorBeginOverlap
  (params (OtherActor :type Actor%20Object%20Reference)))

(event EventTick
  (params (DeltaSeconds :type Float%20%28single-precision%29))
  (if (not (Variables|Default|GetbInitCameras))
    (bind _returnvalue (Actor|GetActorOfClass "/Game/Blueprints/Stage/BP_RaceManager.BP_RaceManager_C"))
    (if (== (Utilities|Array|Length (Variables|/Script/gff_08.RaceManager|GetBoats _returnvalue)) 4)
      (for _array_element (Variables|/Script/gff_08.RaceManager|GetBoats _returnvalue)
        (bind _returnvalue_2 (Game|SpawnActorfromClass "/Game/Blueprints/Camera/BP_Stalker.BP_Stalker_C" (Math|Transform|MakeTransform "0, 0, 0" "0, 0, 0" "1,1,1") "Undefined" 0 0))
        (Variables|/Game/Blueprints/Camera/BP_Stalker.BP_Stalker_C|SetTarget _returnvalue_2 _array_element)
        (Utilities|Array|Add (Variables|Default|GetCameras) _returnvalue_2))
      (bind _outactors (Actor|GetAllActorsOfClass "/Game/Blueprints/Camera/BP_FixedPointCamera.BP_FixedPointCamera_C"))
      (Utilities|Array|AppendArray (Variables|Default|GetCameras) _outactors)
      (Default|EnableCamera (Utilities|Array|Get(acopy) (Variables|Default|GetCameras) (Variables|Default|GetDefaultCameraID)))
      (Variables|Default|SetbInitCameras true))))

(event Input|KeyboardEvents|NumPadOne
  (params (Key :type Key%20Structure :default "None"))
  (:Pressed
    (Default|EnableCamera (Utilities|Array|Get(acopy) (Variables|Default|GetCameras)))))

(event Input|KeyboardEvents|NumPadFive
  (params (Key :type Key%20Structure :default "None"))
  (:Pressed
    (Default|EnableCamera (Utilities|Array|Get(acopy) (Variables|Default|GetCameras) 4))))

(event Input|KeyboardEvents|NumPadSix
  (params (Key :type Key%20Structure :default "None"))
  (:Pressed
    (Default|EnableCamera (Utilities|Array|Get(acopy) (Variables|Default|GetCameras) 5))))

(event Input|KeyboardEvents|NumPadSeven
  (params (Key :type Key%20Structure :default "None"))
  (:Pressed
    (Default|EnableCamera (Utilities|Array|Get(acopy) (Variables|Default|GetCameras) 6))))

(event Input|KeyboardEvents|NumPadEight
  (params (Key :type Key%20Structure :default "None"))
  (:Pressed
    (Default|EnableCamera (Utilities|Array|Get(acopy) (Variables|Default|GetCameras) 7))))

(event Input|KeyboardEvents|NumPadNine
  (params (Key :type Key%20Structure :default "None"))
  (:Pressed
    (Default|EnableCamera (Utilities|Array|Get(acopy) (Variables|Default|GetCameras) 8))))

(event Input|KeyboardEvents|NumPadZero
  (params (Key :type Key%20Structure :default "None"))
  (:Pressed
    (Default|EnableCamera (Utilities|Array|Get(acopy) (Variables|Default|GetCameras) 9))))

(event Input|KeyboardEvents|NumPadTwo
  (params (Key :type Key%20Structure :default "None"))
  (:Pressed
    (Default|EnableCamera (Utilities|Array|Get(acopy) (Variables|Default|GetCameras) 1))))

(event Input|KeyboardEvents|NumPadThree
  (params (Key :type Key%20Structure :default "None"))
  (:Pressed
    (Default|EnableCamera (Utilities|Array|Get(acopy) (Variables|Default|GetCameras) 2))))

(event Input|KeyboardEvents|NumPadFour
  (params (Key :type Key%20Structure :default "None"))
  (:Pressed
    (Default|EnableCamera (Utilities|Array|Get(acopy) (Variables|Default|GetCameras) 3))))

(fn ConstructionScript)