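; Test Blueprint that prints race result data for four players when play begins.
; BeginPlay reads the play data from a GetInstance accessor, then formats and prints each player's index, racer name and three lap times.
; Each player has its own hardcoded print with fixed lap indices, with no loop or check on array length.
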(event EventBeginPlay
  (bind _returnvalue (Class|MyGameInstance|GetInstance))
  (bind _returnvalue_2 (Class|MyGameInstance|GetInstance))
  (bind _returnvalue_3 (Class|MyGameInstance|GetInstance))
  (bind _returnvalue_4 (Class|MyGameInstance|GetInstance))
  (bind _returnvalue_5 (Class|MyGameInstance|GetPlayData _returnvalue_2))
  (bind _returnvalue_6 (Class|MyGameInstance|GetPlayData _returnvalue))
  (bind _returnvalue_7 (Class|MyGameInstance|GetPlayData _returnvalue_3))
  (bind _returnvalue_8 (Class|MyGameInstance|GetPlayData _returnvalue_4))
  (bind _player1data (Variables|/Script/gff_08.AllRacersGamePlayDataObject|GetPlayer1Data _returnvalue_7))
  (bind _player2data (Variables|/Script/gff_08.AllRacersGamePlayDataObject|GetPlayer2Data _returnvalue_8))
  (bind _player3data (Variables|/Script/gff_08.AllRacersGamePlayDataObject|GetPlayer3Data _returnvalue_5))
  (bind _player4data (Variables|/Script/gff_08.AllRacersGamePlayDataObject|GetPlayer4Data _returnvalue_6))
  (bind (_playerindex _racername _laptimes) (Utilities|Struct|BreakGamePlayData _player4data))
  (bind (_playerindex_2 _racername_2 _laptimes_2) (Utilities|Struct|BreakGamePlayData _player1data))
  (bind (_playerindex_3 _racername_3 _laptimes_3) (Utilities|Struct|BreakGamePlayData _player2data))
  (bind (_playerindex_4 _racername_4 _laptimes_4) (Utilities|Struct|BreakGamePlayData _player3data))
  (Development|PrintText (Utilities|Text|FormatText "PlayerIndex: {0} PlayerName: {1} LapTimes {2}, {3}, {4}" _playerindex_2 _racername_2 (Utilities|Array|Get(acopy) _laptimes_2) (Utilities|Array|Get(acopy) _laptimes_2 1) (Utilities|Array|Get(acopy) _laptimes_2 2)))
  (Development|PrintText (Utilities|Text|FormatText "PlayerIndex: {0} PlayerName: {1} LapTimes {2}, {3}, {4}" _playerindex_3 _racername_3 (Utilities|Array|Get(acopy) _laptimes_3) (Utilities|Array|Get(acopy) _laptimes_3 1) (Utilities|Array|Get(acopy) _laptimes_3 2)))
  (Development|PrintText (Utilities|Text|FormatText "PlayerIndex: {0} PlayerName: {1} LapTimes {2}, {3}, {4}" _playerindex_4 _racername_4 (Utilities|Array|Get(acopy) _laptimes_4) (Utilities|Array|Get(acopy) _laptimes_4 1) (Utilities|Array|Get(acopy) _laptimes_4 2)))
  (Development|PrintText (Utilities|Text|FormatText "PlayerIndex: {0} PlayerName: {1} LapTimes {2}, {3}, {4}" _playerindex _racername (Utilities|Array|Get(acopy) _laptimes) (Utilities|Array|Get(acopy) _laptimes 1) (Utilities|Array|Get(acopy) _laptimes 2))))

(fn ConstructionScript)