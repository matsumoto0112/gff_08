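; BP_Render is a capture actor that renders an orthographic scene view to a render target and exports it to disk.
; The construction script applies OrthoWidth to both the Camera and the SceneCaptureComponent2D, keeping their widths matched.
; The CaptureAndExport event reapplies that width, triggers a manual CaptureScene, then exports the capture's texture target using the Filepath and Filename variables.
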(event Custom|CaptureAndExport
  (CallFunction|UpdateSceneCaptureSetting (Variables|Default|GetOrthoWidth))
  (CallFunction|TakeCapture)
  (CallFunction|ExportSceneTexture (Variables|Default|GetFilepath) (Variables|Default|GetFilename)))

(event EventBeginPlay)

(event Collision|EventActorBeginOverlap
  (params (OtherActor :type Actor%20Object%20Reference)))

(fn ConstructionScript
  (CallFunction|UpdateSceneCaptureSetting (Variables|Default|GetOrthoWidth)))

(fn UpdateSceneCaptureSetting
  (params (OrthoWidth :type Float%20%28single-precision%29))
  (Class|CameraComponent|SetOrthoWidth (Variables|Default|GetCamera) OrthoWidth)
  (Variables|/Script/Engine.SceneCaptureComponent2D|SetOrthoWidth (Variables|Default|GetSceneCaptureComponent2D) OrthoWidth))

(fn TakeCapture
  (Rendering|SceneCapture|CaptureScene (Variables|Default|GetSceneCaptureComponent2D) :!class /Script/Engine.SceneCaptureComponent2D))

(fn ExportSceneTexture
  (params (Filepath :type String) (Filename :type String))
  (Rendering|ExportRenderTarget (Variables|/Script/Engine.SceneCaptureComponent2D|GetTextureTarget (Variables|Default|GetSceneCaptureComponent2D)) Filepath Filename))