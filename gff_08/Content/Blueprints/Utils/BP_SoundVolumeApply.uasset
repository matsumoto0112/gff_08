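; Utility Blueprint that applies the player's saved volume options to the game's audio.
; ApplySoundVolume reads the Master, BGM and SE volumes from the option data returned by GetInstance and converts them from percentages to multipliers.
; It sets each as an instant sound class override on the SCM_Master sound mix, then pushes that mix.
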(fn ApplySoundVolume
  (bind _returnvalue (Class|MyGameInstance|GetInstance))
  (Audio|SetSoundMixClassOverride 0 "/Game/Sound/SCM_Master.SCM_Master" "/Game/Sound/SC_Master.SC_Master" (/ (Variables|/Script/gff_08.OptionParameter|GetMasterVolume (Class|MyGameInstance|GetOption _returnvalue)) 1e+02) 1.0 0.0 true)
  (Audio|SetSoundMixClassOverride 0 "/Game/Sound/SCM_Master.SCM_Master" "/Game/Sound/BGM/SC_BGM.SC_BGM" (/ (Variables|/Script/gff_08.OptionParameter|GetBGMVolume (Class|MyGameInstance|GetOption _returnvalue)) 1e+02) 1.0 0.0 true)
  (Audio|SetSoundMixClassOverride 0 "/Game/Sound/SCM_Master.SCM_Master" "/Game/Sound/SE/SC_SE.SC_SE" (/ (Variables|/Script/gff_08.OptionParameter|GetSEVolume (Class|MyGameInstance|GetOption _returnvalue)) 1e+02) 1.0 0.0 true)
  (Audio|PushSoundMixModifier 0 "/Game/Sound/SCM_Master.SCM_Master"))