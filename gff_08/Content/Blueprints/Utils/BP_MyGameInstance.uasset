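; Game instance that holds Strix Cloud networking configuration and property maps for multiplayer rooms and their members.
; Init functions set the application ID, master host and ports, and build room properties (capacity, name) and member properties (name, IsStart flag).
; Typed setters update the member property map and push it to the room via SetRoomMember on the user's channel.
; Shutdown stops the Strix network.
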(event EventShutdown
  (Class|StrixBlueprintFunctionLibrary|StopStrixNetwork))

(fn InitializeUserProperty
  (params (UserName :type String))
  (Variables|Default|SetMemberProperties (Class|StrixBlueprintFunctionLibrary|SetBoolProperty (Class|StrixBlueprintFunctionLibrary|SetStringProperty (Utilities|Struct|MakeStrixPropertyMap) "name" UserName) "IsStart" false)))

(fn InitializeProperties
  (Variables|Default|SetApplicationID "8df430d4-a8f7-4e53-98ac-1ea2cbdeeabb")
  (Variables|Default|SetMasterHostName "4f33be0b0d5a2fdd174aa3d1.game.strixcloud.net")
  (Variables|Default|SetHostPort 9122)
  (Variables|Default|SetRoomPort 9123))

(fn InitializeRoomProperties
  (params (Capacity :type Integer) (RoomName :type String))
  (Variables|Default|SetRoomProperties (Class|StrixBlueprintFunctionLibrary|SetStringProperty (Class|StrixBlueprintFunctionLibrary|SetIntProperty (Utilities|Struct|MakeStrixPropertyMap) "capacity" Capacity) "name" RoomName)))

(fn SetStringMemberProperty
  (params (PropertyName :type String) (Value :type String))
  (bind _output_get (Variables|Default|SetMemberProperties (Class|StrixBlueprintFunctionLibrary|SetStringProperty (Variables|Default|GetMemberProperties) PropertyName Value)))
  (bind _instance (CallFunction|GetMyGameInstance))
  (Class|StrixBlueprintFunctionLibrary|SetRoomMember (Variables|/Script/gff_08.PlayUserData|GetChannelID (Class|MyGameInstance|GetUserData _instance)) _output_get))

(fn SetIntMemberProperty
  (params (PropertyName :type String) (Value :type Integer))
  (bind _output_get (Variables|Default|SetMemberProperties (Class|StrixBlueprintFunctionLibrary|SetIntProperty (Variables|Default|GetMemberProperties) PropertyName Value)))
  (bind _instance (CallFunction|GetMyGameInstance))
  (Class|StrixBlueprintFunctionLibrary|SetRoomMember (Variables|/Script/gff_08.PlayUserData|GetChannelID (Class|MyGameInstance|GetUserData _instance)) _output_get))

(fn SetBoolMemberProperty
  (params (PropertyName :type String) (Value :type Boolean))
  (bind _output_get (Variables|Default|SetMemberProperties (Class|StrixBlueprintFunctionLibrary|SetBoolProperty (Variables|Default|GetMemberProperties) PropertyName Value)))
  (bind _instance (CallFunction|GetMyGameInstance))
  (Class|StrixBlueprintFunctionLibrary|SetRoomMember (Variables|/Script/gff_08.PlayUserData|GetChannelID (Class|MyGameInstance|GetUserData _instance)) _output_get))